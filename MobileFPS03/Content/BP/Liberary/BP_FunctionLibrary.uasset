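; A Blueprint function library with a bullet spread helper that returns a random 2D offset as separate X and Y values.
; It picks a random angle around a full circle and a random radius, then converts them with degree-based cosine and sine.
; The radius limit is the tangent of MaxProjectileDistance multiplied by MaxSpreadAngle, so the two inputs appear swapped relative to their names.
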(fn `FL_BulletSpread`
  (params (MaxSpreadAngle :type "Float (double-precision)" :default 5.0) (MaxProjectileDistance :type "Float (double-precision)" :default 100000000.0))
  (returns (BulletSpread :type "Vector2D Structure"))
  (locals (Angel :type "Float (double-precision)" :default 0.0) (Displacement :type "Float (double-precision)" :default 0.0))
  (set `local.Angel` (`KismetMathLibrary.RandomFloatInRange` 0.0 360.0))
  (set `local.Displacement` (`KismetMathLibrary.RandomFloatInRange` 0.0 (* (`KismetMathLibrary.DegTan` MaxProjectileDistance) MaxSpreadAngle)))
  (return (`KismetMathLibrary.MakeVector2D` (* (`local.Displacement`) (`KismetMathLibrary.DegCos` (`local.Angel`))) (* (`local.Displacement`) (`KismetMathLibrary.DegSin` (`local.Angel`))))))