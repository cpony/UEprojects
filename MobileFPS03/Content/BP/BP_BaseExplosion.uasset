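; BP_BaseExplosion is an explosion actor that pushes and damages its surroundings, then expires after a few seconds.
; On BeginPlay it fires its RadialForce impulse, sets its lifespan and applies minor radial damage over that component's radius.
; Actors overlapping the ParticleSystem take heavier point damage, directed opposite to the explosion's velocity.
; An owner-exclusion check exists but is disconnected, so the owner is not filtered from that damage.
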(event `self.ReceiveBeginPlay`
  (`RadialForceComponent.FireImpulse` (`self.RadialForce`))
  (`self.SetLifeSpan` 5.0)
  (`GameplayStatics.ApplyRadialDamage` :`BaseDamage` 0.5 :`Origin` (`SceneComponent.K2_GetComponentLocation` (`self.DefaultSceneRoot`)) :`DamageRadius` (`RadialForceComponent.Radius` (`self.RadialForce`)) :`DamageCauser` null :`InstigatedByController` null))

(event `self.ParticleSystem.OnComponentBeginOverlap`
  (params (OverlappedComponent :type "PrimitiveComponent Object Reference") (OtherActor :type "Actor Object Reference") (OtherComp :type "PrimitiveComponent Object Reference") (OtherBodyIndex :type Integer) (bFromSweep :type Boolean) (SweepResult :type "HitResult Structure (by ref)"))
  (`GameplayStatics.ApplyPointDamage` OtherActor 30.0 (* (`KismetMathLibrary.Normal` (`self.GetVelocity`)) -1.0) SweepResult))

(fn `UserConstructionScript`)