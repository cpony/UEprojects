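; BP_BaseWeapon is a base gun that manages fire modes, magazine and chamber rounds, and creates the main UI.
; Montages paced by RPM drive firing, then chamber a round on blend-out and repeat for burst or full auto.
; Each shot launches a projectile toward the owner's look-at point, or along the muzzle at extreme yaw or close range.
; A debug-drawn spread trace accompanies shots, with its result unused.
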(event `Server5`
  (`self.Mu5`))

(event `self.ReceiveTick`
  (params (DeltaSeconds :type "Float (single-precision)"))
  (`KismetSystemLibrary.PrintString` (`KismetStringLibrary.Conv_IntToString` (`self.RoundsinMag`)) true true (struct :`G` 0.66 :`B` 1.0 :`A` 1.0) 0.0)
  (`KismetSystemLibrary.PrintString` (`KismetStringLibrary.Conv_IntToString` (`self.RoundsinChamber`)) true true (struct :`G` 0.66 :`B` 1.0 :`A` 1.0) 0.0))

(event `/Game/BP/BPI_Weapons.FirePressed`
  (if (> (`self.RoundsinChamber`) 0)
    (`self.FireProjectile`)))

(event `Mu5`)

(event `self.ReceiveBeginPlay`
  (bind _returnvalue (`|CreateWidget` "/Game/BP/UI/MainUI.MainUI_C" (`GameplayStatics.GetPlayerController` 0)))
  (bind _output_get (set `self.MainUI` _returnvalue))
  (`UserWidget.AddToViewport` _output_get 0))

(event `FirePressedLocal,dont use`)

(event `/Game/BP/BPI_Weapons.GetWeapon`
  (params (OwningCharacter :type "/Game/ThirdPersonCPP/Blueprints/ThirdPersonCharacter Object Reference"))
  (set `self.Owning Character` OwningCharacter)
  (`PrimitiveComponent.SetSimulatePhysics` (`self.SkeletalMesh`) false)
  (`PrimitiveComponent.SetCollisionEnabled` (`self.SkeletalMesh`) "NoCollision")
  (set `self.AimBaseLineOffset` (- (`KismetAnimationLibrary.K2_DistanceBetweenTwoSocketsAndMapRange` (`self.SkeletalMesh`) "Root" "RTS_World" "Sight" "RTS_World") 13.5)))

(event `WeaponFire`
  (bind _owning_character (`self.Owning Character`))
  (bind _roundsinchamber (`self.RoundsinChamber`))
  (bind _returnvalue_location (`KismetMathLibrary.BreakTransform` (`self.GetTransform` _owning_character)))
  (bind _returnvalue_location_2 (`KismetMathLibrary.BreakTransform` (`SceneComponent.GetSocketTransform` (`self.SkeletalMesh`) "Muzzle" "RTS_World")))
  (bind (_returnvalue_location_3 _returnvalue_rotation _returnvalue_scale) (`KismetMathLibrary.BreakTransform` (`SceneComponent.GetSocketTransform` (`self.SkeletalMesh`) "Muzzle" "RTS_World")))
  (bind _returnvalue (`KismetMathLibrary.SelectVector` (`KismetMathLibrary.GetForwardVector` (`SceneComponent.GetSocketRotation` (`self.SkeletalMesh`) "Muzzle")) (`KismetMathLibrary.Normal` (- (`/Game/ThirdPersonCPP/Blueprints/ThirdPersonCharacter.Look at Point` (`self.Owning Character`)) (`SceneComponent.GetSocketLocation` (`self.SkeletalMesh`) "Muzzle"))) (or (>= (`KismetMathLibrary.Abs` (`/Game/ThirdPersonCPP/Blueprints/ThirdPersonCharacter.Yaw` _owning_character)) 90.0) (<= (`KismetMathLibrary.Abs` (`KismetMathLibrary.VSize` (- _returnvalue_location (`/Game/ThirdPersonCPP/Blueprints/ThirdPersonCharacter.Look at Point` (`self.Owning Character`))))) 300.0))))
  (bind _returnvalue_2 (`KismetMathLibrary.Conv_VectorToRotator` _returnvalue))
  (`|VariableSetRef` _roundsinchamber (- _roundsinchamber 1))
  (bind _returnvalue_3 (`|SpawnActorFromClass` "/Game/BP/BP_BaseProjectile02.BP_BaseProjectile02_C" (`KismetMathLibrary.MakeTransform` _returnvalue_location_3 _returnvalue_rotation (* _returnvalue_scale 5.0)) "AlwaysSpawn" "OverrideRootScale" null null))
  (set `MovementComponent.Velocity` (* _returnvalue (`self.MuzzleVelocity`)) (`FPSProjectile.ProjectileMovementComponent` _returnvalue_3))
  (bind _bulletspread (`/Game/BP/Liberary/BP_FunctionLibrary.FL_BulletSpread` (`self.MaxSpreadAngle`) (`self.MaxProjectileDistance`)))
  (`KismetSystemLibrary.LineTraceSingle` :`Start` _returnvalue_location_2 :`End` (+ _returnvalue_location_2 (+ (* (`KismetMathLibrary.GetForwardVector` _returnvalue_2) (`self.MaxProjectileDistance`)) (* (`KismetMathLibrary.GetRightVector` _returnvalue_2) (`KismetMathLibrary.BreakVector2D` _bulletspread)) (* (`KismetMathLibrary.GetUpVector` _returnvalue_2) (`.Y` (`KismetMathLibrary.BreakVector2D` _bulletspread))))) :`TraceChannel` "TraceTypeQuery1" :`DrawDebugType` "ForDuration" :`DrawTime` 20.0))

(event `RepeatFire`
  (switch `/Game/BP/EFireMode` (`self.FireMode`) :!label _label
    (:`NewEnumerator1`
      (`/Engine/EditorBlueprintResources/StandardMacros.DoOnce` false :!label _label_2
        (:`Completed`
          (`|PlayMontage` (`Character.Mesh` (`self.Owning Character`)) "/Game/MyAnimations/A_2HW_ADS_Fire_Montage.A_2HW_ADS_Fire_Montage" (/ (`self.RPM`) 200.0)
            (:`then`
              (`|PlayMontage` (`self.SkeletalMesh`) "/Game/MyAnimations/SK_FPGun_Skeleton_Sequence_Montage.SK_FPGun_Skeleton_Sequence_Montage" (/ (`self.RPM`) 200.0)
                (:`then`
                  (`self.WeaponFire` :!label _label_3))))
            (:`OnBlendOut`
              (`self.Chambering`)
              (goto _label_2 :!via `Reset`))))))
    (:`NewEnumerator2`
      (`|PlayMontage` (`Character.Mesh` (`self.Owning Character`)) "/Game/MyAnimations/A_2HW_ADS_Fire_Montage.A_2HW_ADS_Fire_Montage" (/ (`self.RPM`) 200.0)
        (:`then`
          (`|PlayMontage` (`self.SkeletalMesh`) "/Game/MyAnimations/SK_FPGun_Skeleton_Sequence_Montage.SK_FPGun_Skeleton_Sequence_Montage" (/ (`self.RPM`) 200.0)
            (:`then`
              (`/Engine/EditorBlueprintResources/StandardMacros.IncrementInt` (`self.Brusts`)
                (:`  `
                  (goto _label_3))))))
        (:`OnBlendOut`
          (`self.Chambering`)
          (`self.ShouldRepeatCheck`))))
    (:`NewEnumerator3`
      (`|PlayMontage` (`Character.Mesh` (`self.Owning Character`)) "/Game/MyAnimations/A_2HW_ADS_Fire_Montage.A_2HW_ADS_Fire_Montage" (/ (`self.RPM`) 200.0)
        (:`then`
          (`|PlayMontage` (`self.SkeletalMesh`) "/Game/MyAnimations/SK_FPGun_Skeleton_Sequence_Montage.SK_FPGun_Skeleton_Sequence_Montage" (/ (`self.RPM`) 200.0)
            (:`then`
              (goto _label_3))))
        (:`OnBlendOut`
          (`self.Chambering`)
          (`self.ShouldRepeatCheck`))))))

(event `FireProjectile`
  (set `self.Firing` true)
  (goto _label))

(event `FireReleased`
  (set `self.Firing` false)
  (set `self.Brusts` 0))

(event `WeaponToggleFireMode`
  (if (> (`KismetArrayLibrary.Array_Length` (`self.AvaliableFireMode`)) 1)
    (bind _nextitem (`/Game/BP/Liberary/MyMacroLibrary.GetArrayNextItem` (`self.AvaliableFireMode`) (`self.FireMode`))
      (:`Out`
        (bind _output_get (set `self.FireMode` _nextitem))
        (bind _returnvalue (`|GetEnumeratorNameAsString` _output_get))
        (`KismetSystemLibrary.PrintString` _returnvalue)
        (set `self.FireModeString` _returnvalue)))
    (else
      (`KismetSystemLibrary.PrintString` "NoFireMode"))))

(event `MagReloadDone`
  (params (RoundsLoaded :type Integer))
  (set `self.RoundsinMag` RoundsLoaded))

(fn `Chambering`
  (bind _roundsinmag (`self.RoundsinMag`))
  (bind _roundsinchamber (`self.RoundsinChamber`))
  (if (> (`self.RoundsinMag`) 0)
    (`|VariableSetRef` _roundsinmag (- _roundsinmag 1))
    (`|VariableSetRef` _roundsinchamber (+ _roundsinchamber 1))))

(fn `GetWeaponPanelInfo`
  (returns (BaseWeapon :type "/Game/BP/BP_BaseWeapon Object Reference") (WeaponType :type "/Game/BP/EWeaponType Enum"))
  (return self (`self.WeaponType`)))

(fn `ShouldRepeatCheck`
  (if (select `/Game/BP/EFireMode` (`self.FireMode`) :`NewEnumerator2` (and (`self.Firing`) (> (`self.RoundsinChamber`) 0) (< (`self.Brusts`) 3)) :`NewEnumerator3` (and (`self.Firing`) (> (`self.RoundsinChamber`) 0)))
    (`self.RepeatFIre`)))

(fn `UserConstructionScript`)