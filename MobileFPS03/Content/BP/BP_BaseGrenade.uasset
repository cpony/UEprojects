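; Base grenade actor that explodes on a three-second fuse and deals slight damage to actors it touches.
; A BeginPlay timer fires Detonate, which chains through Serve1 and Mu1 (names suggest server and multicast events) to spawn BP_BaseExplosion at its transform and destroy itself.
; Static mesh overlaps apply point damage to any actor except the owner, using the reversed velocity as hit direction.
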(event `Serve1`
  (`self.Mu1`))

(event `self.ReceiveBeginPlay`
  (`KismetSystemLibrary.K2_SetTimerDelegate` (delegate `Detonate`) 3.0))

(event `Mu1`
  (`|SpawnActorFromClass` "/Game/BP/BP_BaseExplosion.BP_BaseExplosion_C" (`self.GetTransform`) "Undefined" "OverrideRootScale" null null)
  (`self.K2_DestroyActor`))

(event `Detonate`
  (`self.Serve1`))

(event `self.StaticMesh.OnComponentBeginOverlap`
  (params (OverlappedComponent :type "PrimitiveComponent Object Reference") (OtherActor :type "Actor Object Reference") (OtherComp :type "PrimitiveComponent Object Reference") (OtherBodyIndex :type Integer) (bFromSweep :type Boolean) (SweepResult :type "HitResult Structure (by ref)"))
  (if (!= (`self.GetOwner`) OtherActor)
    (`GameplayStatics.ApplyPointDamage` OtherActor 0.3 (* (`KismetMathLibrary.Normal` (`self.GetVelocity`)) -1.0) SweepResult)))

(fn `UserConstructionScript`)